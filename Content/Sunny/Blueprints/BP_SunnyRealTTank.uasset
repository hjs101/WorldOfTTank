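; BP_SunnyRealTTank is a tank vehicle Blueprint that drives turret and gun poses through its animation Blueprint.
; BeginPlay caches the ABP_SunnyRealTank instance, and two events write turret angle and gun elevation to it.
; GetTurretAngle computes an interpolated, actor-relative yaw toward player pawn 0.
; Tick is empty, the aiming and wheel-speed calls are disconnected, and the GunElevation function is an empty stub.
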(event `SetTurretRotation`
  (params (TurretAngle :type "Float (double-precision)"))
  ;[1 1 1] Set turret angle
  (set `/Game/Sunny/SunnyTank/ABP_SunnyRealTank.TurretAngle` TurretAngle (`self.Anim Instance`)))

(event `SetGunElevation`
  (params (GunAngle :type "Float (double-precision)"))
  ;[1 1 1] Set gun elevation
  (set `/Game/Sunny/SunnyTank/ABP_SunnyRealTank.GunElevation` GunAngle (`self.Anim Instance`)))

(event `self.ReceiveBeginPlay`
  (bind _asabp_sunny_real_tank (cast `/Game/Sunny/SunnyTank/ABP_SunnyRealTank` (`SkeletalMeshComponent.GetAnimInstance` (`self.Mesh`))))
  (set `self.Anim Instance` _asabp_sunny_real_tank))

(event `self.ReceiveTick`
  (params (DeltaSeconds :type "Float (single-precision)")))

(fn `GetTurretAngle`
  (params (`Interp Speed` :type "Float (double-precision)"))
  (returns (Yaw :type "Float (double-precision)"))
  (bind (_returnvalue_roll _returnvalue_pitch _returnvalue_yaw) (`KismetMathLibrary.BreakRotator` (`self.K2_GetActorRotation`)))
  (bind (_returnvalue_roll_2 _returnvalue_pitch_2 _returnvalue_yaw_2) (`KismetMathLibrary.BreakRotator` (`KismetMathLibrary.FindLookAtRotation` (`self.K2_GetActorLocation`) (`self.K2_GetActorLocation` (`GameplayStatics.GetPlayerPawn` 0)))))
  (return (.yaw (`KismetMathLibrary.RInterpTo` (`KismetMathLibrary.MakeRotator` 0.0 0.0 (`self.Angle`)) (`KismetMathLibrary.MakeRotator` 0.0 0.0 (- _returnvalue_yaw_2 _returnvalue_yaw)) (`GameplayStatics.GetWorldDeltaSeconds`) (`local.Interp Speed`)))))

(fn `GunElevation`)

(fn `UserConstructionScript`)