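; Sunny tank Blueprint that creates dynamic body and track materials on its mesh at construction.
; SetSpeed passes a speed to WheelSpeed on the stored ABP_SunnyRealTank animation instance, but the code that assigns that reference is disconnected.
; Possession, input mapping and camera pitch limit logic are also disconnected, and BeginPlay and SetWheelSmokeIntensity are empty.
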(event `SetSpeed`
  (params (Speed :type "Float (double-precision)"))
  ;[1 1 1] Set wheel speed
  (set `/Game/Sunny/SunnyTank/ABP_SunnyRealTank.WheelSpeed` Speed (`self.Anim Instance`)))

(event `self.ReceiveBeginPlay`)

(fn `SetWheelSmokeIntensity`
  (params (Intensity :type "Float (double-precision)")))

(fn `UserConstructionScript`
  (bind _mesh (`self.Mesh`))
  (bind _returnvalue (`PrimitiveComponent.CreateDynamicMaterialInstance` _mesh 0 null "None"))
  (set `self.BodyMaterial` _returnvalue)
  (bind _returnvalue_2 (`PrimitiveComponent.CreateDynamicMaterialInstance` _mesh 1 null "None"))
  (set `self.TracksMaterial` _returnvalue_2))